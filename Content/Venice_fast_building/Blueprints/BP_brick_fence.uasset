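; BP_brick_fence is a procedural modular brick fence builder for placing fences of adjustable length in a level.
; Its construction script adds one static mesh section in one of three Fence styles every 300 units along negative Y.
; Toggles add pillars at the start, at the end and between sections.
; Options override the wall material from the WallMATs array and switch between two forged railing materials; the event graph is empty.
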(fn `UserConstructionScript`
  (bind _output (`|GetArrayItem` (`self.Wall_MATs`) (`KismetMathLibrary.Conv_ByteToInt` (`self.Wall_MAT`))))
  (if (`self.Pillar_at_start`)
    (bind _returnvalue (`AddComponent|NODE_AddStaticMeshComponent-5`))
    (if (`self.Wall_or_Brck_MAT`)
      (`PrimitiveComponent.SetMaterial` _returnvalue 0 _output)))
  (for _index (range 1 (+ (`self.Length`) 1))
    (if (and (`self.Along_fence`) (> _index 1) (< _index (+ (`self.Length`) 1)))
      (bind _returnvalue_2 (`KismetMathLibrary.MakeTransform` (`KismetMathLibrary.MakeVector` 0.0 (* (- _index 1) -300.0))))
      (bind _returnvalue_3 (`AddComponent|NODE_AddStaticMeshComponent-0` :`RelativeTransform` _returnvalue_2)))
    (if (`self.Wall_or_Brck_MAT`)
      (`PrimitiveComponent.SetMaterial` _returnvalue_3 0 _output))
    (switch `/Game/Venice_fast_building/Blueprints/lists_structs/E_brick_fences` (`self.fence`)
      (:`NewEnumerator0`
        (bind _returnvalue_4 (`AddComponent|NODE_AddStaticMeshComponent-1` :`RelativeTransform` _returnvalue_2)))
      (:`NewEnumerator1`
        (bind _returnvalue_5 (`AddComponent|NODE_AddStaticMeshComponent-2` :`RelativeTransform` _returnvalue_2)))
      (:`NewEnumerator2`
        (bind _returnvalue_6 (`AddComponent|NODE_AddStaticMeshComponent-3` :`RelativeTransform` _returnvalue_2))))
    (if (`self.Wall_or_Brck_MAT`)
      (`PrimitiveComponent.SetMaterial` _returnvalue_4 0 _output)
      (`PrimitiveComponent.SetMaterial` _returnvalue_5 0 _output)
      (`PrimitiveComponent.SetMaterial` _returnvalue_6 0 _output))
    (if (`self.1_or_2`)
      (`PrimitiveComponent.SetMaterial` _returnvalue_4 2 "/Game/Venice_fast_building/Materials/MI_forged_railing_03.MI_forged_railing_03")
      (`PrimitiveComponent.SetMaterial` _returnvalue_5 2 "/Game/Venice_fast_building/Materials/MI_forged_railing_03.MI_forged_railing_03")
      (`PrimitiveComponent.SetMaterial` _returnvalue_6 2 "/Game/Venice_fast_building/Materials/MI_forged_railing_03.MI_forged_railing_03")
      (else
        (`PrimitiveComponent.SetMaterial` _returnvalue_4 2 "/Game/Venice_fast_building/Materials/MI_forged_railing_05.MI_forged_railing_05")
        (`PrimitiveComponent.SetMaterial` _returnvalue_5 2 "/Game/Venice_fast_building/Materials/MI_forged_railing_05.MI_forged_railing_05")
        (`PrimitiveComponent.SetMaterial` _returnvalue_6 2 "/Game/Venice_fast_building/Materials/MI_forged_railing_05.MI_forged_railing_05"))))
  (if (`self.Pillar_at_end`)
    (bind _returnvalue_7 (`AddComponent|NODE_AddStaticMeshComponent-4` :`RelativeTransform` (`KismetMathLibrary.MakeTransform` (`KismetMathLibrary.MakeVector` 0.0 (* (`self.Length`) -300.0)))))
    (if (`self.Wall_or_Brck_MAT`)
      (`PrimitiveComponent.SetMaterial` _returnvalue_7 0 (`|GetArrayItem` (`self.Wall_MATs`) (`KismetMathLibrary.Conv_ByteToInt` (`self.Wall_MAT`)))))))