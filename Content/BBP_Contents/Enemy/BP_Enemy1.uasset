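; BP_Enemy1 is an enemy Blueprint that plays hit feedback when damaged.
; Tick polls the SpawnDamage flag and calls CreateHitEffect, which clears it and spawns a random Boom, Pow or Bang effect at a random offset from the enemy.
; Each effect is followed by a world camera shake.
; GetState exposes MState, and ReturnCanAnim always returns false.
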(event `self.ReceiveBeginPlay`)

(event `self.ReceiveTick`
  (params (DeltaSeconds :type "Float (single-precision)"))
  (if (`self.spawnDamage`)
    (`self.Create Hit Effect`)))

(fn `Create Hit Effect`
  (bind _returnvalue (+ (`self.K2_GetActorLocation`) (`KismetMathLibrary.RandomFloatInRange` 50.0 100.0)))
  (set `self.spawnDamage` false)
  (switch `int` (`KismetMathLibrary.RandomInteger` 3)
    (:`0`
      (`NiagaraFunctionLibrary.SpawnSystemAtLocation` (`self.Effect_Boom`) _returnvalue))
    (:`1`
      (`NiagaraFunctionLibrary.SpawnSystemAtLocation` (`self.Effect_Pow`) _returnvalue))
    (:`2`
      (`NiagaraFunctionLibrary.SpawnSystemAtLocation` (`self.Effect_Bang`) _returnvalue)))
  (`GameplayStatics.PlayWorldCameraShake` "/Game/BBP_Contents/Camera/HitCameraShake.HitCameraShake_C"))

(fn `Get State`
  (returns (NewParam :type "EEnemyState Enum"))
  (return (`self.mState`)))

(fn `ReturnCanAnim`
  (returns (CanAnim :type Boolean))
  (return false))

(fn `UserConstructionScript`)